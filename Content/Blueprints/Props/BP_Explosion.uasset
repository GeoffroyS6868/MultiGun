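; BP_Explosion is a short-lived explosion actor that plays effects and damages what it touches.
; On BeginPlay it spawns the NS_Explosion Niagara system with a Size parameter, plays a sound at its location, and destroys itself after a brief delay.
; Actors that begin overlapping its Sphere receive a fixed hit through the BPI_BeingHit interface's BeingHitMessage, if they implement it.
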(event OnComponentBeginOverlap(Sphere)
  (params (OverlappedComponent :type Primitive%20Component%20Object%20Reference) (OtherActor :type Actor%20Object%20Reference) (OtherComp :type Primitive%20Component%20Object%20Reference) (OtherBodyIndex :type Integer) (bFromSweep :type Boolean) (SweepResult :type Hit%20Result%20Structure%20%28by%20ref%29))
  ;[0.03854 0.03854 0.03854] Check explosion overlapping actors
  (if (Utilities|DoesObjectImplementInterface OtherActor "/Game/Blueprints/Core/Interface/BPI_BeingHit.BPI_BeingHit_C")
    (Class|BPIBeingHit|BeingHit(Message) OtherActor 100)))

(event EventBeginPlay
  ;[0.04271 0.04271 0.04271] BeginPlay
  (bind _returnvalue (Niagara|SpawnSystematLocation "/Game/Assets/VFX/NS_Explosion.NS_Explosion" (Transformation|GetActorLocation)))
  (Niagara|SetNiagaraVariable(Float) _returnvalue "Size" 3.0)
  (Audio|PlaySoundatLocation "/Game/StarterContent/Audio/Explosion01.Explosion01" (Transformation|GetActorLocation) "0, 0, 0" 1.0 1.0 0.0 "/Game/Assets/Sounds/SA_Main.SA_Main" 0 0 0)
  (Utilities|FlowControl|Delay 1.5)
  (Actor|DestroyActor))

(fn ConstructionScript)