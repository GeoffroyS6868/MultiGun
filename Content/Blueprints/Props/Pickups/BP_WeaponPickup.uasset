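; Weapon pickup prop that the player can interact with to equip a weapon.
; On BeginPlay it writes the weapon name into its interact feedback widget.
; Interact passes the weapon, the pickup itself and the current magazine to the player's EquipWeapon.
; InteractWidget shows the prompt and uses a retriggerable delay to hide it shortly after calls stop, so no explicit hide call is needed.
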(event EventBeginPlay
  (bind _aswbp_interact_feed_back (Utilities|Casting|CastToWBP_InteractFeedBack (UserInterface|GetWidget (Variables|Default|GetWidget))))
  (Default|UpdateWidget _aswbp_interact_feed_back (Utilities|Text|ToText(Name) (Variables|Default|GetWeaponName)))
  (|CallParentFunction))

(event Collision|EventActorBeginOverlap
  (params (OtherActor :type Actor%20Object%20Reference))
  (|CallParentFunction OtherActor) ; This node is disabled and will not be called.\nDrag off pins to build functionality.
)

(event EventTick
  (params (DeltaSeconds :type Float%20%28single-precision%29))
  (|CallParentFunction DeltaSeconds) ; This node is disabled and will not be called.\nDrag off pins to build functionality.
)

(event EventInteract
  (params (Player :type BP%20Multiplayer%20Character%20Object%20Reference))
  (Default|EquipWeapon Player (Variables|Default|GetWeaponToPickup) self (Variables|Default|GetCurrentMagazine)))

(event EventInteractWidget
  (Rendering|SetVisibility (Variables|Default|GetWidget) true false)
  (Utilities|FlowControl|RetriggerableDelay 0.15)
  (Rendering|SetVisibility (Variables|Default|GetWidget) false false))

(fn ConstructionScript
  (|CallParentFunction))