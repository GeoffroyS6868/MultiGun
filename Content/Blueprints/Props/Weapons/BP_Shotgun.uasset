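; Shotgun weapon Blueprint that fires a spread of eight hitscan pellets per shot, using one round from the magazine.
; Shoot checks reload, ammo and cooldown, then runs camera-channel line traces with random Y/Z offsets at max range, rotated to the aim.
; Hits send Damage through BPI_BeingHit or spawn surface impacts; BeginPlay's Damage/8 SpecialDamage goes unused here.
; A valid owner gets fire sound, main-character montage and a FireRate-based cooldown reset.
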(event EventBeginPlay
  (Variables|Default|SetSpecialDamage (/ (Variables|Default|GetDamage) 8))
  (|CallParentFunction))

(event EventShoot
  (params (Rotator :type Rotator :default "0, 0, 0") (OwnerLocation :type Vector :default "0, 0, 0"))
  (bind _returnvalue (Components|GetOwner))
  (if (not (Variables|Default|GetIsReloading))
    (bind _ammo (CallFunction|HasAmmo))
    (if _ammo
      (if (Variables|Default|GetCanShoot)
        (Variables|Default|SetCanShoot false)
        (bind _result (Math|Integer|DecrementInt (Variables|Default|GetCurrentMagazine))
          (:%20%20
            (Default|CallCurrentMagazineAmmoUpdated _result)
            (for _index (range 0 7)
              (bind _rotatedvector (CallFunction|RandomizeVector (Math|Vector|MakeVector (* (Math|Conversions|ToFloat(Integer) (Variables|Default|GetRange)) 1e+02) 0.0 0.0)))
              (bind _outhit (Collision|LineTraceByChannel OwnerLocation (+ (Math|Vector|RotateVector _rotatedvector Rotator) OwnerLocation) "TraceTypeQuery2" false (Utilities|Array|MakeArray (Components|GetOwner)) "ForDuration"))
              (Utilities|IsValid (.hitactor _outhit)
                (:Is%20Valid
                  (if (Utilities|DoesObjectImplementInterface (.hitactor _outhit) "/Game/Blueprints/Core/Interface/BPI_BeingHit.BPI_BeingHit_C")
                    (Class|BPIBeingHit|BeingHit(Message) (.hitactor _outhit) (Variables|Default|GetDamage))
                    (else
                      (CallFunction|SpawnImpact (.hitcomponent _outhit) (.location _outhit) (.normal _outhit)))))))
            (Utilities|IsValid _returnvalue
              (:Is%20Valid
                (bind _asbp_main_character (Utilities|Casting|CastToBP_MainCharacter _returnvalue)
                  (:then
                    (Animation|Montage|MontagePlay (Components|SkeletalMesh|GetAnimInstance (Variables|/Game/Blueprints/Character/BP_MainCharacter.BP_MainCharacter_C|GetSkeletalMesh _asbp_main_character)) "/Game/Animations/AM_Shoot.AM_Shoot" 1.0 "MontageLength" 0.0 true))
                  (:CastFailed
                    _))
                (CallFunction|PlayFireSound OwnerLocation)
                (Utilities|FlowControl|Delay (Math|Float|SafeDivide 1.0 (Math|Conversions|ToFloat(Integer) (Variables|Default|GetFireRate))))
                (Variables|Default|SetCanShoot true)))))))))

(fn ConstructionScript
  (|CallParentFunction))

(fn RandomizeVector
  (params (EndVector :type Vector))
  (return (Math|Vector|MakeVector (.x EndVector) (+ (.y EndVector) (Math|Random|RandomFloatinRange -75.0 75.0)) (+ (.z EndVector) (Math|Random|RandomFloatinRange -75.0 75.0)))))