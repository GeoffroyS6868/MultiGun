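; BP_RocketLauncher is a weapon Blueprint whose Shoot event fires BP_RocketBullet rockets.
; A shot requires ammo, no reload in progress and CanShoot, then decrements the magazine and broadcasts the new count.
; The rocket spawns offset forward along the aim rotation, carrying the weapon's Damage and Range.
; The owning BP_MainCharacter plays a shoot montage, fire audio plays, and a delay based on FireRate re-enables shooting.
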(event EventBeginPlay
  (|CallParentFunction) ; This node is disabled and will not be called.\nDrag off pins to build functionality.
)

(event EventShoot
  (params (Rotator :type Rotator :default "0, 0, 0") (OwnerLocation :type Vector :default "0, 0, 0"))
  ;[0.03854 0.03854 0.03854] Shoot
  (if (not (Variables|Default|GetIsReloading))
    (bind _ammo (CallFunction|HasAmmo))
    (if _ammo
      (if (Variables|Default|GetCanShoot)
        (Variables|Default|SetCanShoot false)
        (bind _result (Math|Integer|DecrementInt (Variables|Default|GetCurrentMagazine))
          (:%20%20
            (Default|CallCurrentMagazineAmmoUpdated _result)
            (bind _bullettransform (CallFunction|GetSpawnTransform OwnerLocation Rotator))
            (Game|SpawnActorfromClass "/Game/Blueprints/Props/Munitions/BP_RocketBullet.BP_RocketBullet_C" (Math|Transform|MakeTransform (+ (Math|Vector|RotateVector (Math|Vector|MakeVector 3e+02 0.0 0.0) (.rotation _bullettransform)) (.location _bullettransform)) (.rotation _bullettransform) (.scale _bullettransform)) "Undefined" "MultiplyWithRoot" 0 (Variables|Default|GetDamage) (Variables|Default|GetRange) 0)
            (bind _asbp_main_character (Utilities|Casting|CastToBP_MainCharacter (Components|GetOwner))
              (:then
                (Animation|Montage|MontagePlay (Components|SkeletalMesh|GetAnimInstance (Variables|/Game/Blueprints/Character/BP_MainCharacter.BP_MainCharacter_C|GetSkeletalMesh _asbp_main_character)) "/Game/Animations/AM_Shoot.AM_Shoot" 1.0 "MontageLength" 0.0 true))
              (:CastFailed
                _))
            (CallFunction|PlayFireSound OwnerLocation)
            (Utilities|FlowControl|Delay (Math|Float|SafeDivide 1.0 (Math|Conversions|ToFloat(Integer) (Variables|Default|GetFireRate))))
            (Variables|Default|SetCanShoot true)))))))

(fn ConstructionScript
  (|CallParentFunction))