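; BP_WinningZone is an actor that marks the level's winning zone and completes the level when the player reaches it carrying documents.
; On BeginPlay it feeds its location, lowered slightly in Z, to the NSWinningZone Niagara effect as the spawn position.
; When BP_MainCharacter overlaps the sphere with HasDocuments set, it calls FinishedLevel on the BP_SilentSpectreInstance game instance.
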(event OnComponentBeginOverlap(Sphere)
  (params (OverlappedComponent :type Primitive%20Component%20Object%20Reference) (OtherActor :type Actor%20Object%20Reference) (OtherComp :type Primitive%20Component%20Object%20Reference) (OtherBodyIndex :type Integer) (bFromSweep :type Boolean) (SweepResult :type Hit%20Result%20Structure%20%28by%20ref%29))
  (bind _asbp_main_character (Utilities|Casting|CastToBP_MainCharacter OtherActor))
  (if (Variables|/Game/Blueprints/Character/BP_MainCharacter.BP_MainCharacter_C|GetHasDocuments _asbp_main_character)
    (bind _asbp_silent_spectre_instance (Utilities|Casting|CastToBP_SilentSpectreInstance (Game|GetGameInstance)))
    (Default|FinishedLevel _asbp_silent_spectre_instance)))

(event EventBeginPlay
  (bind _returnvalue (Transformation|GetActorLocation))
  (Class|NiagaraComponent|SetVariablePosition (Variables|Default|GetNS_WinningZone) "SpawnPos" (Math|Vector|MakeVector (.x _returnvalue) (.y _returnvalue) (- (.z _returnvalue) 3e+01))))

(fn ConstructionScript)