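; Multiplayer game mode that tracks connected player controllers and spawns player characters.
; Login, controller swap and logout events maintain the AllPlayers list, with login and logout also telling BP_GS_Multiplayer to update player connections.
; SpawnPlayer destroys any existing pawn, spawns a BP_MultiplayerCharacter at a random PlayerStart's location with zero rotation, and has the controller possess it.
; Nothing in this graph calls SpawnPlayer, and logout handling only applies to BP_FirstPersonPlayerController.
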(event EventPostLogin
  (params (NewPlayer :type Player%20Controller%20Object%20Reference))
  (Utilities|Array|Add (Variables|Default|GetAllPlayers) NewPlayer)
  (bind _asbp_gs_multiplayer (Utilities|Casting|CastToBP_GS_Multiplayer (Game|GetGameState)))
  (Default|UpdatePlayerConnection _asbp_gs_multiplayer))

(event EventOnSwapPlayerControllers
  (params (OldPC :type Player%20Controller%20Object%20Reference) (NewPC :type Player%20Controller%20Object%20Reference))
  (Utilities|Array|RemoveItem (Variables|Default|GetAllPlayers) OldPC)
  (Utilities|Array|Add (Variables|Default|GetAllPlayers) NewPC))

(event EventOnLogout
  (params (ExitingController :type Controller%20Object%20Reference))
  (bind _asbp_first_person_player_controller (Utilities|Casting|CastToBP_FirstPersonPlayerController ExitingController))
  (Utilities|Array|RemoveItem (Variables|Default|GetAllPlayers) _asbp_first_person_player_controller)
  (bind _asbp_gs_multiplayer (Utilities|Casting|CastToBP_GS_Multiplayer (Game|GetGameState)))
  (Default|UpdatePlayerConnection _asbp_gs_multiplayer))

(fn ConstructionScript)

(fn FindRandomPlayerStart
  (bind _outactors (Actor|GetAllActorsOfClass "/Script/Engine.PlayerStart"))
  (return (Math|Transform|MakeTransform (Transformation|GetActorLocation (Utilities|Array|Get(acopy) _outactors (Math|Random|RandomIntegerinRange 0 (- (Utilities|Array|Length _outactors) 1)))) "0, 0, 0" "1.000000,1.000000,1.000000")))

(fn SpawnPlayer
  (params (PlayerController :type Player%20Controller%20Object%20Reference))
  (bind _returnvalue (Pawn|GetControlledPawn PlayerController))
  (Utilities|IsValid _returnvalue
    (:Is%20Valid
      (Actor|DestroyActor _returnvalue))
    (:Is%20Not%20Valid
      _))
  (bind _returnvalue_2 (Game|SpawnActorfromClass "/Game/Blueprints/Character/BP_MultiplayerCharacter.BP_MultiplayerCharacter_C" (Spawning|FindRandomPlayerStart) "Undefined" "MultiplyWithRoot" 0 0))
  (Pawn|Possess PlayerController _returnvalue_2))