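; Multiplayer game state that runs the match countdown and ends the match.
; Once enough players connect it sets the replicated timer, whose RepNotify refreshes every HUD and, on authority, re-triggers a one-second decrement, forming the countdown loop.
; At zero, RPC events show the scoreboards, wait, then reset players in the game instance, open the main menu and destroy the session.
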(event Custom|UpdatePlayerConnection
  ;[0.04688 0.04688 0.04688] Update Player Connection
  (if (>= (Class|GameplayStatics|GetNumPlayerStates) (Variables|Default|GetMinimumRequiredPlayer))
    (Utilities|FlowControl|DoOnce false
      (:Completed
        (Variables|Default|SetMatchTimeCountdown 600)))))

(event Custom|MatchCountdown
  ;[0.04271 0.04271 0.04271] Match Count Down
  (Utilities|FlowControl|Delay 1.0)
  (Variables|Default|SetMatchTimeCountdown (- (Variables|Default|GetMatchTimeCountdown) 1)))

(event Custom|RPC_FinishScreen
  ;[0.04688 0.04688 0.04688] FinishScreen
  (bind _foundwidgets (Widget|GetAllWidgetsOfClass "/Game/Blueprints/Widget/Game/WBP_ScoreBoard.WBP_ScoreBoard_C" false))
  (for _array_element _foundwidgets
    (Widget|SetVisibility _array_element "Visible"))
  (Utilities|FlowControl|Delay 1e+01)
  (bind _asbp_multigun_instance (Utilities|Casting|CastToBP_MultigunInstance (Game|GetGameInstance)))
  (Default|ResetPlayers _asbp_multigun_instance)
  (Game|OpenLevel(byName) "MainMenu")
  (|DestroySession (Game|GetPlayerController 0)))

(event Custom|RPC_Server_FinishScreen
  (CallFunction|RPCFinishScreen))

(fn ConstructionScript)

(fn OnRepMatchTimeCountdown
  (CallFunction|UpdateMatchCountDownWidget)
  (Networking|SwitchHasAuthority
    (:Authority
      (if (== (Variables|Default|GetMatchTimeCountdown) 600)
        (CallFunction|MatchCountdown)
        (elif (<= (Variables|Default|GetMatchTimeCountdown) 0)
          (CallFunction|RPCServerFinishScreen)
          (else
            (CallFunction|MatchCountdown)))))))

(fn UpdateMatchCountDownWidget
  (bind _foundwidgets (Widget|GetAllWidgetsOfClass "/Game/Blueprints/Widget/Game/WBP_HUD.WBP_HUD_C" false))
  (for _array_element _foundwidgets
    (Default|UpdateCountDown (Variables|/Game/Blueprints/Widget/Game/WBP_HUD.WBP_HUD_C|GetGameHUD _array_element) (Variables|Default|GetMatchTimeCountdown))))