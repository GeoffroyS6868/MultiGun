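; Game instance for a multiplayer game that tracks kill and death counts and handles connection failures.
; Network and travel errors both return to the MainMenu level.
; AddKilltoPlayer increments the victim's and killer's entries in name-keyed Deaths and Kills maps through events named as server RPCs.
; It then pushes both maps to every WBP_ScoreBoard widget it finds.
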(event Custom|RPC_Server_AddKillToPlayerMap
  (params (PlayerName :type String))
  (bind _kills (Variables|Multiplayer|GetKills))
  ;[1 1 1] Add Kill To Player Map
  (if (Utilities|Map|Contains (Variables|Multiplayer|GetKills) PlayerName)
    (Utilities|Map|Add _kills PlayerName (+ (.Value (Utilities|Map|Find _kills PlayerName)) 1))
    (else
      (Utilities|Map|Add (Variables|Multiplayer|GetKills) PlayerName 1))))

(event Custom|RPC_Server_AddDeathToPlayerMap
  (params (PlayerName :type String))
  (bind _deaths (Variables|Multiplayer|GetDeaths))
  ;[1 1 1] Add Death To Player Map
  (if (Utilities|Map|Contains (Variables|Multiplayer|GetDeaths) PlayerName)
    (Utilities|Map|Add _deaths PlayerName (+ (.Value (Utilities|Map|Find _deaths PlayerName)) 1))
    (else
      (Utilities|Map|Add (Variables|Multiplayer|GetDeaths) PlayerName 1))))

(event EventHandleNetworkError
  (params (FailureType :type ENetworkFailure%20Enum :default "NetDriverAlreadyExists") (bIsServer :type Boolean))
  ;[1 1 1] Network Error
  (Game|OpenLevel(byName) "MainMenu"))

(event EventHandleTravelError
  (params (FailureType :type ETravelFailure%20Enum :default "NoLevel"))
  ;[1 1 1] Network Error
  (Game|OpenLevel(byName) "MainMenu"))

(event EventAddKilltoPlayer
  (params (PlayerKilled :type String) (PlayerWhoKilled :type String))
  ;[1 1 1] Add Kill to player
  (CallFunction|RPCServerAddDeathtoPlayerMap PlayerKilled)
  (CallFunction|RPCServerAddKilltoPlayerMap PlayerWhoKilled)
  (bind _foundwidgets (Widget|GetAllWidgetsOfClass "/Game/Blueprints/Widget/Multiplayer/Game/WBP_ScoreBoard.WBP_ScoreBoard_C" false))
  (for _array_element _foundwidgets
    (Default|UpdateScoreBoard _array_element (Variables|Multiplayer|GetKills) (Variables|Multiplayer|GetDeaths))))