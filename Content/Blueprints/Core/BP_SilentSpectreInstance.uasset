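; Game instance for Silent Spectre that holds kill and death tallies, unlocked levels and the current level, and returns to MainMenu on network or travel errors.
; AddKilltoPlayer increments per-name Kills and Deaths maps through server RPC-named events, then pushes both maps to every WBP_ScoreBoard widget.
; FinishedLevel unlocks Beach and shows the win menu with UI-only input.
; GetCurrentLevelName maps the current level enum to its map name.
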(event Custom|RPC_Server_AddKillToPlayerMap
  (params (PlayerName :type String))
  (bind _kills (Variables|Default|GetKills))
  ;[1 1 1] Add Kill To Player Map
  (if (Utilities|Map|Contains (Variables|Default|GetKills) PlayerName)
    (Utilities|Map|Add _kills PlayerName (+ (.Value (Utilities|Map|Find _kills PlayerName)) 1))
    (else
      (Utilities|Map|Add (Variables|Default|GetKills) PlayerName 1))))

(event Custom|RPC_Server_AddDeathToPlayerMap
  (params (PlayerName :type String))
  (bind _deaths (Variables|Default|GetDeaths))
  ;[1 1 1] Add Death To Player Map
  (if (Utilities|Map|Contains (Variables|Default|GetDeaths) PlayerName)
    (Utilities|Map|Add _deaths PlayerName (+ (.Value (Utilities|Map|Find _deaths PlayerName)) 1))
    (else
      (Utilities|Map|Add (Variables|Default|GetDeaths) PlayerName 1))))

(event EventHandleNetworkError
  (params (FailureType :type ENetworkFailure%20Enum :default "NetDriverAlreadyExists") (bIsServer :type Boolean))
  ;[1 1 1] Network Error
  (Game|OpenLevel(byName) "MainMenu"))

(event EventHandleTravelError
  (params (FailureType :type ETravelFailure%20Enum :default "NoLevel"))
  ;[1 1 1] Network Error
  (Game|OpenLevel(byName) "MainMenu"))

(event EventAddKilltoPlayer
  (params (PlayerKilled :type String) (PlayerWhoKilled :type String))
  ;[1 1 1] Add Kill to player
  (CallFunction|RPCServerAddDeathtoPlayerMap PlayerKilled)
  (CallFunction|RPCServerAddKilltoPlayerMap PlayerWhoKilled)
  (bind _foundwidgets (Widget|GetAllWidgetsOfClass "/Game/Blueprints/Widget/Multiplayer/Game/WBP_ScoreBoard.WBP_ScoreBoard_C" false))
  (for _array_element _foundwidgets
    (Default|UpdateScoreBoard _array_element (Variables|Default|GetKills) (Variables|Default|GetDeaths))))

(fn FinishedLevel
  (bind _returnvalue (Game|GetPlayerController 0))
  (if (== (Utilities|Array|FindItem (Variables|Default|GetAvailableLevels) "NewEnumerator1") -1)
    (Utilities|Array|Add (Variables|Default|GetAvailableLevels) "NewEnumerator1"))
  (Viewport|RemoveAllWidgets)
  (bind _returnvalue_2 (UserInterface|CreateWidget "/Game/Blueprints/Widget/Menu/WBP_WinMenu.WBP_WinMenu_C" _returnvalue))
  (Variables|/Script/Engine.PlayerController|SetbShowMouseCursor _returnvalue true)
  (Input|SetInputModeUIOnly _returnvalue _returnvalue_2 "DoNotLock" false)
  (UserInterface|Viewport|AddtoViewport _returnvalue_2 0))

(fn GetCurrentLevelName
  (switch Utilities|FlowControl|Switch|SwitchonE_Levels (Variables|Default|GetCurrentLevel)
    (:NewEnumerator0
      (return "DesertVillage"))
    (:NewEnumerator1
      (return "Beach"))))